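; BP_TextRender is a world text label that appears only while something overlaps the actor.
; The TextRender component is hidden on BeginPlay, then shown or hidden by the actor begin and end overlap events, with no filter on the overlapping actor.
; Every Tick rotates the whole actor so its X axis follows the direction from the player camera to the text.
; The Trigger component's own overlap events are empty.
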(event `self.ReceiveBeginPlay`
  (`SceneComponent.SetVisibility` (`self.TextRender`) false false))

(event `self.ReceiveTick`
  (params (DeltaSeconds :type "Float (single-precision)"))
  (`self.K2_SetActorRotation` (`KismetMathLibrary.MakeRotFromX` (- (`SceneComponent.K2_GetComponentLocation` (`self.TextRender`)) (`self.K2_GetActorLocation` (`GameplayStatics.GetPlayerCameraManager` 0))))))

(event `self.ReceiveActorBeginOverlap`
  (params (OtherActor :type "Actor Object Reference"))
  (`SceneComponent.SetVisibility` (`self.TextRender`) true false))

(event `self.Trigger.OnComponentBeginOverlap`
  (params (OverlappedComponent :type "PrimitiveComponent Object Reference") (OtherActor :type "Actor Object Reference") (OtherComp :type "PrimitiveComponent Object Reference") (OtherBodyIndex :type Integer) (bFromSweep :type Boolean) (SweepResult :type "HitResult Structure (by ref)")))

(event `self.Trigger.OnComponentEndOverlap`
  (params (OverlappedComponent :type "PrimitiveComponent Object Reference") (OtherActor :type "Actor Object Reference") (OtherComp :type "PrimitiveComponent Object Reference") (OtherBodyIndex :type Integer)))

(event `self.ReceiveActorEndOverlap`
  (params (OtherActor :type "Actor Object Reference"))
  (`SceneComponent.SetVisibility` (`self.TextRender`) false false))

(fn `UserConstructionScript`)